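; BP_Chair is a world chair Blueprint that triggers a non-looping book-opening start-game animation once it has an owner.
; BeginPlay starts a looping timer that polls for a valid owner several times a second.
; When one appears, the timer clears itself and, if the referenced object in NewVar is valid, plays the animation on that object's skeletal mesh.
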(event `self.ReceiveBeginPlay`
  (bind _returnvalue (`KismetSystemLibrary.K2_SetTimerDelegate` (delegate `CustomEvent`) 0.3 true))
  (set `self.NewVar_0` _returnvalue))

(event `CustomEvent`
  (bind _newvar (`self.NewVar`))
  (`/Engine/EditorBlueprintResources/StandardMacros.IsValid` (`self.GetOwner`)
    (:`Is Valid`
      (`KismetSystemLibrary.K2_ClearAndInvalidateTimerHandle` (`self.NewVar_0`))
      (`/Engine/EditorBlueprintResources/StandardMacros.IsValid` _newvar
        (:`Is Valid`
          (`SkeletalMeshComponent.PlayAnimation` (`/Game/Blueprints/World/BP_Book.SkeletalMesh` _newvar) "/Game/Meshs/Animations/OpenBook_Startgame_Animation.OpenBook_Startgame_Animation" false))))))

(fn `UserConstructionScript`)