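; BP_StartPlayer is a player character or pawn that drives a book-style start screen with UI-only input and a visible cursor.
; On BeginPlay it caches the controller and the camera tagged Camera2, then after a short delay opens BP_Book on its Main page.
; OpenNewPage plays the first-page animation forward or in reverse via play rate and position, shows the requested page when opening, and blends the view to that camera.
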(event `self.ReceiveBeginPlay`
  (`|ExecutionSequence`
    (:`then_0`
      (bind _asplayer_controller (cast `PlayerController` (`self.GetController`)))
      (`WidgetBlueprintLibrary.SetInputMode_UIOnlyEx` _asplayer_controller null)
      (set `PlayerController.bShowMouseCursor` true _asplayer_controller)
      (set `self.Player Controller` _asplayer_controller))
    (:`then_1`
      (`KismetSystemLibrary.Delay` 0.6)
      (bind _outactors (`GameplayStatics.GetAllActorsOfClass` "/Game/Blueprints/World/BP_Book.BP_Book_C"))
      (bind _output (`|GetArrayItem` _outactors))
      (set `self.Book` _output)
      (bind _skeletalmesh (`/Game/Blueprints/World/BP_Book.SkeletalMesh` _output))
      (`SkeletalMeshComponent.PlayAnimation` _skeletalmesh "/Game/Meshs/Animations/OpenBook_Animation.OpenBook_Animation" false)
      (`SkeletalMeshComponent.SetPlayRate` _skeletalmesh 0.4)
      (`Book.ShowPages` _output "Main"))
    (:`then_2`
      (bind _outactors_2 (`GameplayStatics.GetAllActorsOfClass` "/Script/CinematicCamera.CineCameraActor"))
      (for _array_element _outactors_2
        (if (`self.ActorHasTag` _array_element "Camera2")
          (set `self.Second Camera` _array_element))))))

(event `OpenNewPage`
  (params (bIsOpen :type Boolean) (EnumPage :type "EPages Enum" :default "Main"))
  (bind _book (`self.Book`)
    (:`then`
      (if bIsOpen
        (`Book.ShowPages` _book EnumPage))
      (bind _skeletalmesh (`/Game/Blueprints/World/BP_Book.SkeletalMesh` _book))
      (`SkeletalMeshComponent.PlayAnimation` _skeletalmesh "/Game/Meshs/Animations/OpenBook_FirstPage_Animation.OpenBook_FirstPage_Animation" false)
      (`SkeletalMeshComponent.SetPlayRate` _skeletalmesh (`KismetMathLibrary.SelectFloat` 0.8 -1.0 bIsOpen))
      (`SkeletalMeshComponent.SetPlayRate` _skeletalmesh (`KismetMathLibrary.SelectFloat` 0.8 -1.0 bIsOpen))
      (`SkeletalMeshComponent.SetPosition` _skeletalmesh (`KismetMathLibrary.SelectFloat` 0.0 1.0 bIsOpen) false)
      (`PlayerController.SetViewTargetWithBlend` (`self.Player Controller`) (`self.Second Camera`) 0.6 "VTBlend_Linear" 0.0 false))
    (:`else`)))

(fn `UserConstructionScript`)