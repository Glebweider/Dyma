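; BP_Bottle is an interactable alcohol bottle that gives the player a temporary post-process effect and slower walking.
; Construction pulls its mesh and effect duration from DT_AlkoBottles by row name.
; StartInteract shows the player's post-process component and starts a timer that later hides it.
; Both steps relay through RPS_Interact to Multi_Interact, which hides the bottle and toggles walk speed, destroying the actor on the second call.
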(event `InteractInterface.StartInteract`
  (params (InteractPlayer :type "Character Object Reference"))
  (if (not (`self.bIsDelete`))
    (`KismetSystemLibrary.K2_SetTimerDelegate` (delegate `CustomEvent`) (`self.Duration`))
    (`SceneComponent.SetVisibility` (`self.GetComponentByClass` InteractPlayer "/Script/Engine.PostProcessComponent") true false)
    (`self.RPS_Interact` InteractPlayer)))

(event `RPS_Interact`
  (params (Target :type "Character Object Reference"))
  (`self.Multi_Interact` Target))

(event `CustomEvent`
  (`SceneComponent.SetVisibility` (`self.GetComponentByClass` (stale `InteractInterface.StartInteract` InteractPlayer) "/Script/Engine.PostProcessComponent") false false)
  (`self.RPS_Interact` (stale `InteractInterface.StartInteract` InteractPlayer)))

(event `Multi_Interact`
  (params (Target :type "Character Object Reference"))
  (bind _returnvalue (`self.GetComponentByClass` Target "/Script/Engine.CharacterMovementComponent"))
  (`self.SetActorHiddenInGame` true)
  (bind _output_get (set `self.bIsDelete` (not (`self.bIsDelete`))))
  (if _output_get
    (set `CharacterMovementComponent.MaxWalkSpeed` 180.0 _returnvalue)
    (else
      (set `CharacterMovementComponent.MaxWalkSpeed` 250.0 _returnvalue)
      (`self.K2_DestroyActor`))))

(fn `UserConstructionScript`
  (bind _returnvalue (`|GetDataTableRow` "/Game/Blueprints/Tables/DT_AlkoBottles.DT_AlkoBottles" (`self.Row Name`))
    (:`then`
      (bind (_mesh _duration) (break `AlkoBottleData` _returnvalue))
      (`StaticMeshComponent.SetStaticMesh` (`self.StaticMesh`) _mesh)
      (set `self.Duration` _duration))))