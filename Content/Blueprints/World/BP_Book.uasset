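; BP_Book is an animated skeletal-mesh book that serves as a menu, with Main, Settings and Customization pages on widget components.
; BeginPlay registers each page's widget components through AddPages, and OpenMainPage reverses the page animation and shows Main.
; The navigation functions reuse one open-book animation, changing play rate sign and, for the second page, start position to control direction.
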(event `self.ReceiveBeginPlay`
  (`self.InitWidgets`))

(event `OpenMainPage`
  (`self.NavToSecondPage` false)
  (`self.ShowPages` "Main"))

(fn `InitWidgets`
  (`self.AddPages` "Main" (`|MakeArray` (`self.FirstPage`)))
  (`self.AddPages` "Settings" (`|MakeArray` (`self.SettingsRightPage`) (`self.SettingsLeftPage`)))
  (`self.AddPages` "Customization" (`|MakeArray` (`self.CustomizationRightPage`) (`self.CustomizationLeftPage`))))

(fn `NavToFirstPage`
  (bind _skeletalmesh (`self.SkeletalMesh`))
  (`SkeletalMeshComponent.PlayAnimation` _skeletalmesh "/Game/Meshs/Animations/OpenBook_FirstPage_Animation.OpenBook_FirstPage_Animation" false)
  (`SkeletalMeshComponent.SetPlayRate` _skeletalmesh -1.0))

(fn `NavToSecondPage`
  (params (bIsForward :type Boolean))
  (bind _skeletalmesh (`self.SkeletalMesh`))
  (`SkeletalMeshComponent.PlayAnimation` _skeletalmesh "/Game/Meshs/Animations/OpenBook_FirstPage_Animation.OpenBook_FirstPage_Animation" false)
  (`SkeletalMeshComponent.SetPlayRate` _skeletalmesh (select `bool` bIsForward :`false` -1.0 :`true` 1.0 :!type "Float (single-precision)"))
  (`SkeletalMeshComponent.SetPosition` _skeletalmesh (`KismetMathLibrary.SelectFloat` 0.0 0.57 bIsForward) false))

(fn `UserConstructionScript`)